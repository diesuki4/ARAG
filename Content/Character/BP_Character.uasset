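; BP_Character is a character Blueprint that lets the player swap between a sword and a bow with the 1 and 2 keys.
; Both keys call EquipWeapon, which unequips and destroys any valid current weapon, then spawns the requested class.
; CombatComponent holds the current weapon reference, and each weapon handles its own Equip and Unequip, with Equip receiving the character.
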(event `Key|One`
  (params (Key :type "Key Structure"))
  (:`Pressed`
    (`self.Equip Weapon` "/Game/Character/Weapons/BP_SwordA.BP_SwordA_C")))

(event `Key|Two`
  (params (Key :type "Key Structure"))
  (:`Pressed`
    (`self.Equip Weapon` "/Game/Character/Weapons/BP_BowA.BP_BowA_C")))

(fn `Equip Weapon`
  (params (WeaponClass :type "ARWeaponBase Class Reference"))
  (bind _currentweapon (`ARCombatComponent.CurrentWeapon` (`self.CombatComponent`)))
  (`/Engine/EditorBlueprintResources/StandardMacros.IsValid` _currentweapon
    (:`Is Valid`
      (`ARWeaponBase.Unequip` _currentweapon)
      (`self.K2_DestroyActor` _currentweapon)
      (set `ARCombatComponent.CurrentWeapon` null (`self.CombatComponent`)))
    (:`Is Not Valid`
      _))
  (bind _returnvalue (`|SpawnActorFromClass` WeaponClass (`KismetMathLibrary.MakeTransform` (0.0 0.0 0.0)) "Undefined" "OverrideRootScale" null null))
  (bind _output_get (set `ARCombatComponent.CurrentWeapon` _returnvalue (`self.CombatComponent`)))
  (`ARWeaponBase.Equip` _output_get self))

(fn `UserConstructionScript`)